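; Game state that tracks survivor (customer) spawns, escapes and kills, along with the player's score, and pushes them to the HUD.
; Each kill scores its base value times a kill streak multiplier, then increments the multiplier and restarts its window.
; A looping timer advances that window, resets the multiplier when it expires and updates the HUD bar.
; Game over polls until no enemy characters remain, then disables input and shows the Game Over screen.
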(event EventBeginPlay
  ;[1 1 1] Begin Play Event
  (bind _returnvalue (Utilities|Time|SetTimerbyFunctionName 0 "UpdateKillStreak" 0.1 true)) ; Turn on our Event for Updating our Kill Streak
  (Variables|Default|SetKillStreakTimer _returnvalue) ; Store our Timer Handle
  (Variables|Default|SetMultiplierTimer (Variables|Default|GetMultiplierMaxBetweenKills)) ; Set our Multiplier Timer to the max so it starts off empty and at 1
)

(event EventHandleGameOver
  (bind _returnvalue (Game|GetPlayerController 0))
  ;[1 1 1] Handle the Game Over Event
  (bind _alive (CallFunction|CheckforSurvivors :!label _label)) ; Check if any customers are still alive
  (if _alive ; Any Alive?
    (Utilities|FlowControl|Delay 2.0) ; Wait 2 seconds before checking again
    (goto _label)
    (else
      (Input|DisableInput (Game|GetPlayerCharacter 0) (Game|GetPlayerController 0)) ; Disable Player Input
      (bind _returnvalue_2 (UserInterface|CreateWidget "/Game/Blueprints/UI/GameOverScreen.GameOverScreen_C")) ; Create the Game Over Widget
      (UserInterface|Viewport|AddtoViewport _returnvalue_2 0) ; Add Game Over Widget to the Screen
      (Input|SetInputModeUIOnly _returnvalue 0 false) ; Set our input to UI
      (Variables|/Script/Engine.PlayerController|SetbShowMouseCursor _returnvalue true) ; Show the Players Mouse Cursor
    )))

(event EventSurvivorEscaped
  ;[1 1 1] Handle a Customer Escaping
  (CallFunction|HandleSurvivorEscaped))

(event EventSurvivorKilled
  (params (BaseValue :type Integer))
  ;[1 1 1] Handle a Customer being Serviced (Killed)
  (CallFunction|HandleSurvivorKilled BaseValue))

(event EventSurvivorSpawned
  ;[1 1 1] Handle a Customer Spawning into the game
  (CallFunction|HandleSurvivorSpawned))

(fn ConstructionScript)

(fn HandleSurvivorEscaped
  (bind _output_get (Variables|Default|SetNumAlive (- (Variables|Default|GetNumAlive) 1))) ; Remove 1 from our Customers Alive Variable
  (Class|PlayerHUDInterface|UpdateSurvivorsRemaining(Message) (Variables|Default|GetPlayerHudWidget) _output_get) ; Update the HUD with our new number
  (bind _output_get_2 (Variables|Default|SetNumEscaped (+ (Variables|Default|GetNumEscaped) 1))) ; Add 1 to our Customers Serviced Variable
  (Class|PlayerHUDInterface|UpdateSurvivorsEscaped(Message) (Variables|Default|GetPlayerHudWidget) _output_get_2) ; Update the HUD with our new number
)

(fn HandleSurvivorKilled
  (params (BaseValue :type Integer))
  (CallFunction|UpdateScore BaseValue) ; Update the Players Score Variable
  (bind _output_get (Variables|Default|SetNumAlive (- (Variables|Default|GetNumAlive) 1))) ; Remove 1 from our Customers Alive Variable
  (Class|PlayerHUDInterface|UpdateSurvivorsRemaining(Message) (Variables|Default|GetPlayerHudWidget) _output_get) ; Update our HUD with the new Number
  (bind _output_get_2 (Variables|Default|SetNumKilled (+ (Variables|Default|GetNumKilled) 1))) ; Add 1 to our Customers Serviced Variable
  (Class|PlayerHUDInterface|UpdateSurvivorsKilled(Message) (Variables|Default|GetPlayerHudWidget) _output_get_2) ; Update the HUD with the new number
  (Variables|Default|SetKillStreakMultiplier (+ (Variables|Default|GetKillStreakMultiplier) 1)) ; Add 1 to our Kill Streak Multiplier
  (Variables|Default|SetMultiplierTimer 0.0) ; Set our countdown timer for the multiplier back to 0
  (Class|PlayerHUDInterface|UpdateScore(Message) (Variables|Default|GetPlayerHudWidget) (Variables|Default|GetPlayerScore)) ; Update the Players Score on the HUD
)

(fn HandleSurvivorSpawned
  (bind _output_get (Variables|Default|SetNumAlive (+ (Variables|Default|GetNumAlive) 1))) ; Add 1 to our Customers Alive variable
  (Class|PlayerHUDInterface|UpdateSurvivorsRemaining(Message) (Variables|Default|GetPlayerHudWidget) _output_get) ; Update the HUD with the new Number
)

(fn UpdateKillStreak
  (bind _output_get (Variables|Default|SetMultiplierTimer (Math|Float|Clamp(Float) (+ (Variables|Default|GetMultiplierTimer) 0.1) 0.0 (Variables|Default|GetMultiplierMaxBetweenKills)))) ; Add 0.1 to our Multiplier Counter and Clamp between 0 and the Max
  (if (>= _output_get (Variables|Default|GetMultiplierMaxBetweenKills)) ; Has our Timer gone too long?
    (Variables|Default|SetKillStreakMultiplier 1) ; Set the multiplier back to 1
  )
  (Class|PlayerHUDInterface|UpdateKillStreak(Message) (Variables|Default|GetPlayerHudWidget) (Variables|Default|GetKillStreakMultiplier)) ; Update our Kill Streak Number on the HUD
  (Class|PlayerHUDInterface|UpdateKillStreakTimer(Message) (Variables|Default|GetPlayerHudWidget) (- 1.0 (/ (Variables|Default|GetMultiplierTimer) (Variables|Default|GetMultiplierMaxBetweenKills)))) ; Update our Timer Bar for the Kill Streak on the HUD
)

(fn UpdateScore
  (params (BaseValue :type Integer))
  (bind _output_get (LocalVariables|SetLocalValue BaseValue)) ; Set the Base Value Locally
  (Variables|Default|SetPlayerScore (+ (* _output_get (Variables|Default|GetKillStreakMultiplier)) (Variables|Default|GetPlayerScore))) ; Set the new Player Score based on the Local Score value and the Multiplier
)

(fn CheckforSurvivors
  (bind _outactors (Actor|GetAllActorsOfClass "/Game/People/EnemyCharacter.EnemyCharacter_C")) ; Get all of our Enemy Characters in the level right now
  (if (> (Utilities|Array|Length _outactors) 0) ; Are there any?
    (return true) ; Return Yes
    (else
      (return false) ; Return No
    )))