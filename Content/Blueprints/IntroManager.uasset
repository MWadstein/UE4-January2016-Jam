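; IntroManager scripts an intro sequence in which a crowd yells, then a growing button triggers their destruction.
; On BeginPlay it shuffles the level's skeletal mesh actors and, at random intervals, starts each PeopleAnimBP yelling at a random speed.
; A delayed, re-arming timer scales up the button until a size threshold.
; It then swaps people for destructibles shattered by radius damage, removes designated brushes and relocates the button.
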(event Custom|MakeButtonLarge
  (bind _button (Variables|Default|GetButton))
  (bind _scalemultiple (Variables|Default|GetScaleMultiple))
  (bind _returnvalue (Transformation|GetActorTransform _button))
  (bind _returnvalue_2 (+ (.scale _returnvalue) _scalemultiple))
  (Transformation|SetActorTransform (Variables|Default|GetButton) (Math|Transform|MakeTransform (.location _returnvalue) (.rotation _returnvalue) _returnvalue_2))
  (if (>= (.X (Math|Vector|BreakVector _returnvalue_2)) 0.5)
    (for _array_element (Variables|Default|GetSMs)
      (Utilities|Casting|CastToPeopleAnimBP (Components|SkeletalMesh|GetAnimInstance (Variables|/Script/Engine.SkeletalMeshActor|GetSkeletalMeshComponent _array_element)))
      (bind _returnvalue_3 (Game|SpawnActorfromClass "/Game/People/MaleType1/DM/MaleType1_DA.MaleType1_DA_C" (Transformation|GetWorldTransform (Variables|/Script/Engine.SkeletalMeshActor|GetSkeletalMeshComponent _array_element)) "Undefined" 0 0))
      (Class|DestructibleComponent|ApplyRadiusDamage (Variables|/Script/Engine.DestructibleActor|GetDestructibleComponent _returnvalue_3) 1e+02 (.Location (Math|Transform|BreakTransform (Transformation|GetWorldTransform (Variables|/Script/Engine.SkeletalMeshActor|GetSkeletalMeshComponent _array_element)))) 1e+02 5e+03 true)
      (Actor|DestroyActor _array_element) ; destroy people
    )
    (for _array_element_2 (Variables|Default|GetBrushesToDestroy)
      (Actor|DestroyActor _array_element_2))
    (Transformation|SetActorLocation (Variables|Default|GetButton) "-1420.000000,-6970.000000,35.000000" false false)
    (else
      (bind _returnvalue_4 (Utilities|Time|SetTimerbyFunctionName 0 "MakeButtonLarge" 0.1))
      (Variables|Default|SetTimerHandle _returnvalue_4))))

(event EventBeginPlay
  (bind _returnvalue (Utilities|Time|SetTimerbyFunctionName 0 "MakeButtonLarge" 24.0))
  (Variables|Default|SetTimerHandle _returnvalue)
  (bind _outactors (Actor|GetAllActorsOfClass "/Script/Engine.SkeletalMeshActor"))
  (Variables|Default|SetSMs _outactors)
  (Utilities|Array|Shuffle (Variables|Default|GetSMs))
  (Utilities|FlowControl|Delay (Math|Random|RandomFloatinRange 0.4 2.0) :!label _label)
  (if (Utilities|IsValid (Utilities|Array|Get(acopy) (Variables|Default|GetSMs) (Variables|Default|GetSMIndex)))
    (bind _aspeople_anim_bp (Utilities|Casting|CastToPeopleAnimBP (Components|SkeletalMesh|GetAnimInstance (Variables|/Script/Engine.SkeletalMeshActor|GetSkeletalMeshComponent (Utilities|Array|Get(acopy) (Variables|Default|GetSMs) (Variables|Default|GetSMIndex)))))
      (:then
        (Variables|/Game/People/Animations/PeopleAnimBP.PeopleAnimBP_C|SetYellingSpeed _aspeople_anim_bp (Math|Random|RandomFloatinRange 0.6 1.5))
        (Variables|/Game/People/Animations/PeopleAnimBP.PeopleAnimBP_C|SetIsYelling _aspeople_anim_bp true))
      (:CastFailed
        _))
    (Variables|Default|SetSMIndex (+ (Variables|Default|GetSMIndex) 1))
    (if (not (>= (Variables|Default|GetSMIndex) (Utilities|Array|Length (Variables|Default|GetSMs))))
      (goto _label))))

(fn ConstructionScript)