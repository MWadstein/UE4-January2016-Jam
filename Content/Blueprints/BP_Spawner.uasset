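; Spawner actor that creates waves of AI characters at its own transform.
; SpawnWave stores the wave settings, then loops with a delay until the per-wave count is reached, notifying the GameState of each spawn.
; Each spawn has a small chance to be EnemyType1Char with an attack behavior tree, otherwise a random Characters entry with the standard enemy tree.
; BeginPlay sets a timer for SpawnWave if spawning is already enabled.
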(event Custom|SpawnWave
  (params (NumWaves :type Integer) (WaveDelay :type Float%20%28single-precision%29) (SpawnDelay :type Float%20%28single-precision%29) (SpawnsPerWave :type Integer))
  (bind _returnvalue (Transformation|GetActorTransform))
  (bind _returnvalue_2 (Transformation|GetActorTransform))
  (bind _characters (Variables|Default|GetCharacters))
  ;[1 1 1] Event o handle spawning the customers for this wave
  (Variables|Default|SetNumWavesToSpawn NumWaves) ; Store for later use
  (Variables|Default|SetDelayBetweenWaves WaveDelay) ; Store for later use
  (Variables|Default|SetDelayBetweenSpawns SpawnDelay) ; Store for later use
  (Variables|Default|SetNumSpawnsPerWave SpawnsPerWave) ; Store for later use
  (Variables|Default|SetIsSpawning true) ; Should we be spawning?
  (Variables|Default|SetEnemiesSpawnedThisWave 0) ; Reset our spawn amount back to 0
  (if (== (Math|Random|RandomIntegerinRange 0 9) 3) :!label _label
    (AI|SpawnAIFromClass "/Game/People/EnemyType1/EnemyType1Char.EnemyType1Char_C" "/Game/People/AttackEnemy_BT.AttackEnemy_BT" (.location _returnvalue) (.rotation _returnvalue) false) ; Spawn an Enemy AI
    (else
      (AI|SpawnAIFromClass (Utilities|Array|Get(acopy) _characters (Math|Random|RandomIntegerinRange 0 (- (Utilities|Array|Length _characters) 1))) "/Game/People/Enemy_BT.Enemy_BT" (.location _returnvalue_2) (.rotation _returnvalue_2) false) ; Spawn an Enemy AI
    ))
  (Utilities|FlowControl|Delay (Variables|Default|GetDelayBetweenSpawns)) ; Wait between spawns
  (Variables|Default|SetEnemiesSpawnedThisWave (+ (Variables|Default|GetEnemiesSpawnedThisWave) 1)) ; Add 1 to our enemy spawn count
  (Class|GameStateInterface|SurvivorSpawned(Message) (Game|GetGameState)) ; Tell our GameState we spawned a Customer
  (if (not (>= (Variables|Default|GetEnemiesSpawnedThisWave) (Variables|Default|GetNumSpawnsPerWave))) ; Did we spawn all the customers this wave?
    (goto _label)))

(event EventBeginPlay
  ;[1 1 1] Begin Play
  (if (Variables|Default|GetIsSpawning) ; Have we been told to start spawning?
    (bind _returnvalue (Utilities|Time|SetTimerbyFunctionName 0 "SpawnWave" (Variables|Default|GetDelayBetweenWaves))) ; Turn on the Spawn Event using a Timer
    (Variables|Default|SetSpawnTimerHandle _returnvalue) ; Store the Timer Handle for later
  ))

(fn ConstructionScript)