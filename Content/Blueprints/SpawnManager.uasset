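; Spawn manager that runs the enemy wave rounds across three store floors, starting after a store-closing message and delay.
; A self-rescheduling SpawnWave timer reads the Waves array, treats the Floor vector as per-floor flags, and triggers a random spawner on each flagged floor.
; Each spawn shows widget text and plays a chime plus floor-combination voice line.
; When rounds run out, it signals game over to the GameState.
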(event Custom|StopSpawning
  (Class|KismetSystemLibrary|ClearTimerHandle (Variables|Default|GetTimerHandle)))

(event Custom|StartSpawning
  ;[1 1 1] Start our Spawning Event
  (CallFunction|DestroyHintTexts) ; Destroy the Control Hint Texts
  (bind _returnvalue (Utilities|Time|SetTimerbyFunctionName 0 "SpawnWave" 1.0)) ; Start our Event for Spawning Enemy Waves
  (Variables|Default|SetTimerHandle _returnvalue) ; Store our Timer Handle
)

(event Custom|AnnounceWaveSpawns
  (params (Floors :type Vector))
  ;[1 1 1] Event for Announcing our Wave Spawns
  (Audio|PlaySound2D "/Game/Audio/Announcer/bingbong.bingbong") ; Play the Bing Bong sound
  (Utilities|FlowControl|Delay 2.5) ; Wait for the Sound to Finish
  (CallFunction|AnnounceWaveSpawn Floors) ; Announce The Wave Spawns in Text and Sound
)

(event EventBeginPlay
  ;[1 1 1] Begin Play Event
  (bind _returnvalue (UserInterface|CreateWidget "/Game/Blueprints/UI/WaveSpawnedText.WaveSpawnedText_C")) ; Create our Wave Spawned Text Widget
  (bind _output_get (Variables|Default|SetSpawnTextWidget _returnvalue)) ; Store the Widget for later use
  (UserInterface|Viewport|AddtoViewport _output_get 0) ; Add to our screen
  (bind _outactors (Actor|GetAllActorsOfClass "/Game/Blueprints/BP_Spawner.BP_Spawner_C")) ; DEPRECATED: Get all of our spawners
  (Variables|Default|SetAllSpawnPoints _outactors) ; Store our Spawners in an Array
  (Utilities|Array|Shuffle (Variables|Default|GetAllSpawnPoints)) ; Shuffle our Spawners Array
  (CallFunction|ShuffleFloorSpawners) ; Shuffle the floor Spawner Arrays
  (CallFunction|GivePlayerControl) ; Let our player move
  (CallFunction|PlayStoreClosingMessage)
  (Utilities|FlowControl|Delay 15.0) ; Wait 5 Seconds Before Starting
  (Widget|RemovefromParent (Variables|Default|GetStoreClosingWidget))
  (CallFunction|StartSpawning) ; Start Spawning Enemies
)

(fn ConstructionScript)

(fn ShuffleFloorSpawners
  ;[1 1 1] Shuffle our 3 Floor Spawner Arrays
  (Utilities|Array|Shuffle (Variables|Default|GetFloor1SpawnPoints))
  (Utilities|Array|Shuffle (Variables|Default|GetFloor2SpawnPoints))
  (Utilities|Array|Shuffle (Variables|Default|GetFloor3SpawnPoints)))

(fn SpawnWave
  (bind _floor3spawnpoints (Variables|Default|GetFloor3SpawnPoints))
  (bind _floor1spawnpoints (Variables|Default|GetFloor1SpawnPoints))
  (bind _floor2spawnpoints (Variables|Default|GetFloor2SpawnPoints))
  ;[1 1 1] Our Event for Spawning Enemies
  (if (>= (Variables|Default|GetCurrentWave) (Utilities|Array|Length (Variables|Default|GetWaves))) ; Check for no more waves after this one
    (Class|GameStateInterface|HandleGameOver(Message) (Game|GetGameState)) ; Tell the GameState the game is over
    (else
      (Utilities|FlowControl|Sequence ; Check to see if we have enemies to spawn
        (:then_0
          (if (== (.x (.floor (Utilities|Array|Get(acopy) (Variables|Default|GetWaves) (Variables|Default|GetCurrentWave)))) 1.0) ; Do we have a Floor 1 to spawn?
            (Default|SpawnWave (Utilities|Array|Get(acopy) _floor1spawnpoints (Math|Random|RandomIntegerinRange 0 (- (Utilities|Array|Length _floor1spawnpoints) 1))) (.numwaves (Utilities|Array|Get(acopy) (Variables|Default|GetWaves) (Variables|Default|GetCurrentWave))) (.wavedelay (Utilities|Array|Get(acopy) (Variables|Default|GetWaves) (Variables|Default|GetCurrentWave))) (.spawndelay (Utilities|Array|Get(acopy) (Variables|Default|GetWaves) (Variables|Default|GetCurrentWave))) (.spawnsperwave (Utilities|Array|Get(acopy) (Variables|Default|GetWaves) (Variables|Default|GetCurrentWave)))) ; Tell the Spawner to spawn enemies
          ))
        (:then_1
          (if (== (.y (.floor (Utilities|Array|Get(acopy) (Variables|Default|GetWaves) (Variables|Default|GetCurrentWave)))) 1.0) ; Do we have a Floor 2 to spawn?
            (Default|SpawnWave (Utilities|Array|Get(acopy) _floor2spawnpoints (Math|Random|RandomIntegerinRange 0 (- (Utilities|Array|Length _floor2spawnpoints) 1))) (.numwaves (Utilities|Array|Get(acopy) (Variables|Default|GetWaves) (Variables|Default|GetCurrentWave))) (.wavedelay (Utilities|Array|Get(acopy) (Variables|Default|GetWaves) (Variables|Default|GetCurrentWave))) (.spawndelay (Utilities|Array|Get(acopy) (Variables|Default|GetWaves) (Variables|Default|GetCurrentWave))) (.spawnsperwave (Utilities|Array|Get(acopy) (Variables|Default|GetWaves) (Variables|Default|GetCurrentWave)))) ; Tell the Spawner to spawn enemies
          ))
        (:then_2
          (if (== (.z (.floor (Utilities|Array|Get(acopy) (Variables|Default|GetWaves) (Variables|Default|GetCurrentWave)))) 1.0) ; Do we have a Floor 3 to spawn?
            (Default|SpawnWave (Utilities|Array|Get(acopy) _floor3spawnpoints (Math|Random|RandomIntegerinRange 0 (- (Utilities|Array|Length _floor3spawnpoints) 1))) (.numwaves (Utilities|Array|Get(acopy) (Variables|Default|GetWaves) (Variables|Default|GetCurrentWave))) (.wavedelay (Utilities|Array|Get(acopy) (Variables|Default|GetWaves) (Variables|Default|GetCurrentWave))) (.spawndelay (Utilities|Array|Get(acopy) (Variables|Default|GetWaves) (Variables|Default|GetCurrentWave))) (.spawnsperwave (Utilities|Array|Get(acopy) (Variables|Default|GetWaves) (Variables|Default|GetCurrentWave)))) ; Tell the Spawner to spawn enemies
          ))
        (:then_3
          (Default|ShowSpawnMessage (Variables|Default|GetSpawnTextWidget) (.floor (Utilities|Array|Get(acopy) (Variables|Default|GetWaves) (Variables|Default|GetCurrentWave)))) ; Show our Enemies Spawned Message
          (CallFunction|AnnounceWaveSpawns (.floor (Utilities|Array|Get(acopy) (Variables|Default|GetWaves) (Variables|Default|GetCurrentWave)))) ; Announce the Spawns with Audio
          (bind _output_get (Variables|Default|SetSpawnWaveNum (+ (Variables|Default|GetSpawnWaveNum) 1))) ; Add 1 to our number of waves Spawned this Round
          (if (>= _output_get (.numwaves (Utilities|Array|Get(acopy) (Variables|Default|GetWaves) (Variables|Default|GetCurrentWave)))) ; Did we spawn all the waves?
            (bind _returnvalue (Utilities|Time|SetTimerbyFunctionName 0 "SpawnWave" (+ (.wavedelay (Utilities|Array|Get(acopy) (Variables|Default|GetWaves) (Variables|Default|GetCurrentWave))) (.delayafterlastspawn (Utilities|Array|Get(acopy) (Variables|Default|GetWaves) (Variables|Default|GetCurrentWave)))))) ; Set up our next round of spawns
            (Variables|Default|SetTimerHandle _returnvalue) ; Store our Timer Handle
            (Variables|Default|SetCurrentWave (+ (Variables|Default|GetCurrentWave) 1)) ; Add 1 to our current Round
            (Variables|Default|SetSpawnWaveNum 0) ; set oiur number of waves spawned back to 0
            (else
              (Utilities|Time|SetTimerbyFunctionName 0 "SpawnWave" (.wavedelay (Utilities|Array|Get(acopy) (Variables|Default|GetWaves) (Variables|Default|GetCurrentWave)))) ; Set up our next wave to spawn this round
            )))))))

(fn AnnounceWaveSpawn
  (params (FloorNum :type Vector))
  ;[1 1 1] Which sound do we play based on the Floors that spawn
  (Utilities|FlowControl|Sequence ; Check which floors have spawned
    (:then_0
      (if (== (.x FloorNum) 1.0) ; Set our Floor1 Variable
        (LocalVariables|SetIsFloor1 true)))
    (:then_1
      (if (== (.y FloorNum) 1.0) ; Set our Floor2 Variable
        (LocalVariables|SetIsFloor2 true)))
    (:then_2
      (if (== (.z FloorNum) 1.0) ; Set our Floor3 Variable
        (LocalVariables|SetIsFloor3 true)))
    (:then_3
      (if (LocalVariables|GetIsFloor1) ; Spawn on Floor1?
        (if (LocalVariables|GetIsFloor2) ; And Floor2?
          (if (LocalVariables|GetIsFloor3) ; And Floor3?
            (Audio|PlaySound2D "/Game/Audio/Announcer/floors-123.floors-123") ; Play 1,2, and 3
            (else
              (Audio|PlaySound2D "/Game/Audio/Announcer/floors-12.floors-12") ; Play 1 and 2
            ))
          (elif (LocalVariables|GetIsFloor3)
            (Audio|PlaySound2D "/Game/Audio/Announcer/floors-13.floors-13") ; Play 1 and 3
            (else
              (Audio|PlaySound2D "/Game/Audio/Announcer/floors-1.floors-1") ; Play 1
            )))
        (elif (LocalVariables|GetIsFloor2) ; Spawn on Floor2?
          (if (LocalVariables|GetIsFloor3) ; And Floor3?
            (Audio|PlaySound2D "/Game/Audio/Announcer/floors-23.floors-23") ; Play 2 and 3
            (else
              (Audio|PlaySound2D "/Game/Audio/Announcer/floors-2.floors-2") ; Play 2
            ))
          (elif (LocalVariables|GetIsFloor3)
            (Audio|PlaySound2D "/Game/Audio/Announcer/floors-3.floors-3") ; Play 3
          ))))))

(fn GivePlayerControl
  ;[1 1 1] Give our Player Control
  (Input|EnableInput (Game|GetPlayerCharacter 0) (Game|GetPlayerController 0)))

(fn DestroyHintTexts
  ;[1 1 1] Destroy our Startup Control hint text actors
  (bind _outactors (Actor|GetAllActorsOfClass "/Script/Engine.TextRenderActor"))
  (for _array_element _outactors
    (Actor|DestroyActor _array_element)))

(fn PlayStoreClosingMessage
  (Audio|PlaySound2D "/Game/Audio/Announcer/StoresClosing.StoresClosing" (Variables|/Game/Blueprints/XelaGameState.XelaGameState_C|GetSoundVolume (.AsXela%20Game%20State (Utilities|Casting|CastToXelaGameState (Game|GetGameState)))))
  (bind _returnvalue (UserInterface|CreateWidget "/Game/Blueprints/UI/StoresClosingText.StoresClosingText_C"))
  (bind _output_get (Variables|Default|SetStoreClosingWidget _returnvalue))
  (UserInterface|Viewport|AddtoViewport _output_get 0))